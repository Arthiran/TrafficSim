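; Drivable truck that hitches trailers, with switchable first and third person cameras.
; Input drives the vehicle movement component, while Tick rotates the active camera arm, cab body, steering wheel and dashboard needles.
; A coupler overlap stores the nearby BP_Trailer and shows a widget prompt; keys attach or detach it and toggle lights on both.
; Dynamic materials set paint color at construction and light glow at runtime.
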(event OnComponentBeginOverlap(COupler_Box)
  (params (OverlappedComponent :type Primitive%20Component%20Object%20Reference) (OtherActor :type Actor%20Object%20Reference) (OtherComp :type Primitive%20Component%20Object%20Reference) (OtherBodyIndex :type Integer) (bFromSweep :type Boolean) (SweepResult :type Hit%20Result%20Structure%20%28by%20ref%29))
  ;[1 1 1] OverlapEvents
  (if (Utilities|Enum|Equal(Enum) (Utilities|GetObjectName OtherComp) "Box2")
    (bind _asbp_trailer (Utilities|Casting|CastToBP_Trailer OtherActor))
    (Variables|Default|SetTrailer_Ref _asbp_trailer)
    (Utilities|IsValid (Variables|Default|GetWB_Truck)
      (:Is%20Valid
        ;[1 1 1] SetTextIntoWidget
        (CallFunction|SetWidgetTExt "\"G\" to attach trailer")))))

(event OnComponentEndOverlap(COupler_Box)
  (params (OverlappedComponent :type Primitive%20Component%20Object%20Reference) (OtherActor :type Actor%20Object%20Reference) (OtherComp :type Primitive%20Component%20Object%20Reference) (OtherBodyIndex :type Integer))
  ;[1 1 1] OverlapEvents
  (Variables|Default|SetTrailer_Ref 0)
  (Utilities|IsValid (Variables|Default|GetWB_Truck)
    (:Is%20Valid
      (CallFunction|SetWidgetTExt))))

(event EventTick
  (params (DeltaSeconds :type Float%20%28single-precision%29))
  (bind _returnvalue (Input|AxisValues|GetTurn))
  (bind _springarm_3st (Variables|Default|GetSpringArm_3st))
  (bind _caboffset (Variables|Default|GetCabOffset))
  (bind _steeringwheel (Variables|Default|GetSteeringWheel))
  (bind _springarm1st (Variables|Default|GetSpringArm1St))
  (bind _cameraid (Variables|Other|GetCameraID))
  (bind _vehiclemovement (Variables|Default|GetVehicleMovement))
  (bind _returnvalue_2 (Transformation|GetWorldRotation _caboffset))
  (bind _returnvalue_3 (Utilities|Select :Index _cameraid :Option%200 _springarm1st :Option%201 _springarm_3st))
  (bind _relativerotation (Variables|/Script/Engine.SceneComponent|GetRelativeRotation _returnvalue_3))
  ;[0 0.6314 0] SetCameraRotation
  (Variables|Default|SetDeltaSec DeltaSeconds)
  (Transformation|SetRelativeRotation _returnvalue_3 (Math|Rotator|MakeRotator (.roll _relativerotation) (+ (.pitch _relativerotation) (Class|Actor|GetInputAxisKeyValue)) (+ (.yaw _relativerotation) (Class|Actor|GetInputAxisKeyValue))) false false)
  (Transformation|SetWorldRotation (Variables|Default|GetTruck_Body_01) (Math|Rotator|MakeRotator (.roll _returnvalue_2) (+ (.pitch _returnvalue_2) 2.0) (.yaw _returnvalue_2)) false false)
  (Utilities|FlowControl|Sequence
    (:then_0
      ;[1 1 1] SteeringWheelRotation
      (if (Variables|Default|GetCanDrive?)
        (if (== _returnvalue 0.0)
          (bind _output_get (Variables|Default|SetWheelRotation (Math|Interpolation|FInterpTo (Variables|Default|GetWheelRotation) 0.0 (Variables|Default|GetDeltaSec) 2.0)))
          (Transformation|SetRelativeRotation _steeringwheel (Math|Rotator|MakeRotator _output_get -3e+01 0.0) false false)
          (else
            (bind _output_get_2 (Variables|Default|SetWheelRotation (Math|Interpolation|FInterpTo (Variables|Default|GetWheelRotation) (* _returnvalue 2.4e+02) (Variables|Default|GetDeltaSec) 2.0)))
            (Transformation|SetRelativeRotation _steeringwheel (Math|Rotator|MakeRotator _output_get_2 -3e+01 0.0) false false)))))
    (:then_1
      ;[1 1 1] ArrowRotation
      (Transformation|SetRelativeRotation (Variables|Default|GetTaometerArrow) (Math|Rotator|MakeRotator (- (/ (Class|WheeledVehicleMovementComponent|GetEngineRotationSpeed _vehiclemovement) 2e+01) 115.0) 0.0 0.0) false false)
      (Transformation|SetRelativeRotation (Variables|Default|GetSpeedometerArrow) (Math|Rotator|MakeRotator (- (/ (Class|WheeledVehicleMovementComponent|GetForwardSpeed _vehiclemovement) 1e+01) 115.0) 0.0 0.0) false false))))

(event EventBeginPlay
  ;[1 1 1] AddWidget
  (bind _returnvalue (UserInterface|CreateWidget "/Game/TruckAndTrailers/Blueprints/WB_TruckInfo.WB_TruckInfo_C"))
  (bind _output_get (Variables|Default|SetWB_Truck _returnvalue))
  (UserInterface|Viewport|AddtoViewport _output_get 0)
  ;[1 1 1] CreateDynamicLightMaterial
  (bind _returnvalue_2 (Rendering|Material|CreateDynamicMaterialInstance "/Game/TruckAndTrailers/Materials/Materials/MI_Light_Material.MI_Light_Material" "None" :!class /Script/Engine.KismetMaterialLibrary))
  (bind _output_get_2 (Variables|Default|SetLightMat _returnvalue_2))
  (Rendering|Material|SetMaterial (Variables|Default|GetTruck_Lights) 0 _output_get_2))

(event Input|ActionEvents|InputActionHandbrake
  (params (Key :type Key%20Structure))
  (bind _vehiclemovement (Variables|Default|GetVehicleMovement))
  ;[1 1 1] Wehicle Movement
  (:Pressed
    (Class|WheeledVehicleMovementComponent|SetHandbrakeInput _vehiclemovement true))
  (:Released
    (Class|WheeledVehicleMovementComponent|SetHandbrakeInput _vehiclemovement false)))

(event Input|AxisEvents|InputAxisTurn
  (params (AxisValue :type Float%20%28single-precision%29))
  ;[1 1 1] CustomMovement
  ;[1 1 1] Wehicle Movement
  (Class|WheeledVehicleMovementComponent|SetSteeringInput (Variables|Default|GetVehicleMovement) AxisValue))

(event Input|AxisEvents|InputAxisAcceleration
  (params (AxisValue :type Float%20%28single-precision%29))
  ;[1 1 1] CustomMovement
  ;[1 1 1] Wehicle Movement
  (Class|WheeledVehicleMovementComponent|SetThrottleInput (Variables|Default|GetVehicleMovement) AxisValue))

(event Input|MouseEvents|MouseWheelDown
  (params (Key :type Key%20Structure))
  (bind _springarm_3st (Variables|Default|GetSpringArm_3st))
  ;[1 1 1] CameraZoom
  (:Pressed
    (Variables|/Script/Engine.SpringArmComponent|SetTargetArmLength _springarm_3st (+ (Variables|/Script/Engine.SpringArmComponent|GetTargetArmLength _springarm_3st) 2e+01))))

(event Input|MouseEvents|MouseWheelUp
  (params (Key :type Key%20Structure))
  (bind _springarm_3st (Variables|Default|GetSpringArm_3st))
  ;[1 1 1] CameraZoom
  (:Pressed
    (Variables|/Script/Engine.SpringArmComponent|SetTargetArmLength _springarm_3st (- (Variables|/Script/Engine.SpringArmComponent|GetTargetArmLength _springarm_3st) 2e+01))))

(event Input|KeyboardEvents|R
  (params (Key :type Key%20Structure))
  ;[1 1 1] RestartLevel
  (:Pressed
    (Game|OpenLevel(byName) "Preview")))

(event Input|KeyboardEvents|2
  (params (Key :type Key%20Structure))
  ;[1 1 1] Set3StCameraActive
  (:Pressed
    (Components|Activation|Deactivate (Variables|Default|GetCamera_1st))
    (Components|Activation|SetActive (Variables|Default|GetCamera_3st) true false)
    (Variables|Other|SetCameraID 1)))

(event Input|KeyboardEvents|1
  (params (Key :type Key%20Structure))
  ;[1 1 1] Set1StCameraActive
  (:Pressed
    (Components|Activation|Deactivate (Variables|Default|GetCamera_3st))
    (Components|Activation|SetActive (Variables|Default|GetCamera_1st) true false)
    (Variables|Other|SetCameraID 0)))

(event Input|KeyboardEvents|G
  (params (Key :type Key%20Structure))
  (bind _trailer_ref (Variables|Default|GetTrailer_Ref))
  ;[1 1 1] Attach/DetachTrailer
  (:Pressed
    (Utilities|IsValid _trailer_ref
      (:Is%20Valid
        (if (not (Variables|Default|GetTrailerAttached))
          (Default|AttachTrailer _trailer_ref self)
          (Variables|Default|SetTrailerAttached true)
          (CallFunction|SetWidgetTExt)
          ;[1 1 1] ToggleTrailerLights
          (Default|ToggleLights (Variables|Default|GetTrailer_Ref)))))))

(event Input|KeyboardEvents|L
  (params (Key :type Key%20Structure))
  (bind _lightmat (Variables|Default|GetLightMat))
  (bind _light_f_r (Variables|Default|GetLight_F_R))
  ;[1 1 1] TurnLights
  (:Pressed
    (if (Variables|Default|GetLightOn?)
      (Rendering|Material|SetScalarParameterValue _lightmat "LightIntensity" 1.0 :!class /Script/Engine.MaterialInstanceDynamic)
      (Variables|Default|SetLightOn? false)
      (Rendering|SetVisibility _light_f_r false false)
      (else
        (Rendering|Material|SetScalarParameterValue _lightmat "LightIntensity" 1e+01 :!class /Script/Engine.MaterialInstanceDynamic)
        (Variables|Default|SetLightOn? true)
        (Rendering|SetVisibility _light_f_r true false)))
    ;[1 1 1] ToggleTrailerLights
    (if (Variables|Default|GetTrailerAttached)
      (Default|ToggleLights (Variables|Default|GetTrailer_Ref)))))

(event Input|KeyboardEvents|T
  (params (Key :type Key%20Structure))
  ;[1 1 1] Attach/DetachTrailer
  (:Pressed
    (Default|DetachTrailer (Variables|Default|GetTrailer_Ref))
    (Variables|Default|SetTrailerAttached false)))

(fn ConstructionScript
  ;[1 1 1] CreateTruckMaterial/SetColor
  (bind _returnvalue (Rendering|Material|CreateDynamicMaterialInstance "/Game/TruckAndTrailers/Materials/Materials/MI_Tuck_Material.MI_Tuck_Material" "None" :!class /Script/Engine.KismetMaterialLibrary))
  (bind _output_get (Variables|Default|SetTruckMat _returnvalue))
  (Rendering|Material|SetVectorParameterValue _output_get "CarColor" (Variables|Default|GetTruckColor) :!class /Script/Engine.MaterialInstanceDynamic)
  (Rendering|Material|SetMaterial (Variables|Default|GetTruck_Body_00) 0 (Variables|Default|GetTruckMat)))

(fn SetWidgetTExt
  (params (InText :type Text))
  (Default|SetText (Variables|Default|GetWB_Truck) InText))