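; BP_Trailer is a physics-simulated trailer that hitches to and unhitches from a BP_Truck.
; AttachTrailer grabs it with a physics handle; a shared timeline pulls it to the truck's coupler and moves two boxes vertically, then constrains it to the truck mesh.
; DetachTrailer reverses that timeline, breaks the constraint after a delay and switches off the lights.
; ToggleLights mirrors the truck's light state through a dynamic material and light visibility.
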(event Custom|AttachTrailer
  (params (NewParam :type BP%20Truck%20Object%20Reference))
  (bind _physicshandle (Variables|Default|GetPhysicsHandle))
  ;[1 1 1] SetBoxesRelativeLocation
  (Variables|Default|SetBox1_RelativeLocation (Variables|/Script/Engine.SceneComponent|GetRelativeLocation (Variables|Default|GetBox1)))
  (Variables|Default|SetBox_RelativeLocation (Variables|/Script/Engine.SceneComponent|GetRelativeLocation (Variables|Default|GetBox)))
  (Variables|Default|SetTruckRef NewParam)
  (Utilities|FlowControl|Sequence
    (:then_0
      ;[1 1 1] GrabTrailerToTruck
      (Class|PhysicsHandleComponent|GrabComponentatLocation (Variables|Default|GetPhysicsHandle) (Variables|Default|GetTrailerSK) "Root" (Transformation|GetWorldLocation (Variables|Default|GetDetachConstraint)))
      ;[1 1 1] MoveBoxes
      (bind _newtrack_0 (Timeline|Timeline_0 PlayFromStart)
        (:Update
          ;;[0 1 0.0832] SetLocationToConnect
          (Physics|Components|PhysicsHandle|SetTargetLocation _physicshandle (Math|Vector|MakeVector (.x (Transformation|GetWorldLocation (Variables|/Game/TruckAndTrailers/Blueprints/BP_Truck.BP_Truck_C|GetCoupler (Variables|Default|GetTruckRef)))) (.y (Transformation|GetWorldLocation (Variables|/Game/TruckAndTrailers/Blueprints/BP_Truck.BP_Truck_C|GetCoupler (Variables|Default|GetTruckRef)))) (+ (.z (Transformation|GetWorldLocation (Variables|/Game/TruckAndTrailers/Blueprints/BP_Truck.BP_Truck_C|GetCoupler (Variables|Default|GetTruckRef)))) -4e+01)))
          (Transformation|SetRelativeLocation (Variables|Default|GetBox) (Math|Vector|MakeVector (.x (Variables|Default|GetBox_RelativeLocation)) (.y (Variables|Default|GetBox_RelativeLocation)) (Math|Float|Lerp (.z (Variables|Default|GetBox_RelativeLocation)) (- (.z (Variables|Default|GetBox_RelativeLocation)) -4e+01) _newtrack_0)) true false)
          (Transformation|SetRelativeLocation (Variables|Default|GetBox1) (Math|Vector|MakeVector (.x (Variables|Default|GetBox1_RelativeLocation)) (.y (Variables|Default|GetBox1_RelativeLocation)) (Math|Float|Lerp (.z (Variables|Default|GetBox1_RelativeLocation)) (- (.z (Variables|Default|GetBox1_RelativeLocation)) -4e+01) _newtrack_0)) true false))
        (:Finished
          ;[1 1 1] Release handle and attach constraint(Trailer)
          (Physics|Components|PhysicsHandle|ReleaseComponent _physicshandle)
          (Class|PhysicsConstraintComponent|SetLinearBreakable (Variables|Default|GetDetachConstraint) false 1e+07)
          (bind _asbp_truck (Utilities|Casting|CastToBP_Truck (Components|GetOwner (Variables|/Script/Engine.Actor|GetRootComponent (Variables|Default|GetTruckRef)))))
          (Class|PhysicsConstraintComponent|SetConstrainedComponents (Variables|Default|GetDetachConstraint) (Variables|/Script/PhysXVehicles.WheeledVehicle|GetMesh _asbp_truck) "Root" (Variables|Default|GetTrailerSK) "Root"))))
    (:then_1
      ;[1 1 1] SetMass
      (Class|PrimitiveComponent|SetMassOverrideinKg (Variables|Default|GetTrailerSK) "None" 4e+02 true))
    (:then_2
      ;[1 1 1] CreateDynamicLightMaterial
      (bind _returnvalue (Rendering|Material|CreateDynamicMaterialInstance "/Game/TruckAndTrailers/Materials/Materials/MI_Light_Material.MI_Light_Material" "None" :!class /Script/Engine.KismetMaterialLibrary))
      (bind _output_get (Variables|Default|SetLightMat _returnvalue))
      (Rendering|Material|SetMaterial (Variables|Default|GetMarkerlight_R) 0 _output_get))))

(event Custom|DetachTrailer
  (bind _physicshandle (Variables|Default|GetPhysicsHandle))
  (bind _truckref (Variables|Default|GetTruckRef))
  (bind _box1_relativelocation (Variables|Default|GetBox1_RelativeLocation))
  (bind _box_relativelocation (Variables|Default|GetBox_RelativeLocation))
  (bind _coupler (Variables|/Game/TruckAndTrailers/Blueprints/BP_Truck.BP_Truck_C|GetCoupler _truckref))
  (bind _returnvalue (Transformation|GetWorldLocation _coupler))
  ;[1 1 1] DetachTrailer
  (Utilities|FlowControl|Sequence
    (:then_0
      ;[1 1 1] MoveBoxes
      (bind _newtrack_0 (Timeline|Timeline_0 ReverseFromEnd)
        (:Update
          ;;[0 1 0.0832] SetLocationToConnect
          (Physics|Components|PhysicsHandle|SetTargetLocation _physicshandle (Math|Vector|MakeVector (.x _returnvalue) (.y _returnvalue) (+ (.z _returnvalue) -4e+01)))
          (Transformation|SetRelativeLocation (Variables|Default|GetBox) (Math|Vector|MakeVector (.x _box_relativelocation) (.y _box_relativelocation) (Math|Float|Lerp (.z _box_relativelocation) (- (.z _box_relativelocation) -4e+01) _newtrack_0)) true false)
          (Transformation|SetRelativeLocation (Variables|Default|GetBox1) (Math|Vector|MakeVector (.x _box1_relativelocation) (.y _box1_relativelocation) (Math|Float|Lerp (.z _box1_relativelocation) (- (.z _box1_relativelocation) -4e+01) _newtrack_0)) true false))
        (:Finished
          ;[1 1 1] Release handle and attach constraint(Trailer)
          (Physics|Components|PhysicsHandle|ReleaseComponent _physicshandle)
          (Class|PhysicsConstraintComponent|SetLinearBreakable (Variables|Default|GetDetachConstraint) false 1e+07)
          (bind _asbp_truck (Utilities|Casting|CastToBP_Truck (Components|GetOwner (Variables|/Script/Engine.Actor|GetRootComponent (Variables|Default|GetTruckRef)))))
          (Class|PhysicsConstraintComponent|SetConstrainedComponents (Variables|Default|GetDetachConstraint) (Variables|/Script/PhysXVehicles.WheeledVehicle|GetMesh _asbp_truck) "Root" (Variables|Default|GetTrailerSK) "Root"))))
    (:then_1
      (Utilities|FlowControl|Delay 2.0)
      (Class|PhysicsConstraintComponent|BreakConstraint (Variables|Default|GetDetachConstraint))
      ;[1 1 1] ToggleLights
      (Rendering|Material|SetScalarParameterValue (Variables|Default|GetLightMat) "LightIntensity" 1.0 :!class /Script/Engine.MaterialInstanceDynamic)
      (Rendering|SetVisibility (Variables|Default|GetLight_L) false false))))

(event Custom|ToggleLights
  (bind _light_l (Variables|Default|GetLight_L))
  (bind _lightmat (Variables|Default|GetLightMat))
  ;[1 1 1] ToggleLights
  (if (Variables|/Game/TruckAndTrailers/Blueprints/BP_Truck.BP_Truck_C|GetLightOn? (Variables|Default|GetTruckRef))
    (Rendering|Material|SetScalarParameterValue _lightmat "LightIntensity" 1e+01 :!class /Script/Engine.MaterialInstanceDynamic)
    (Rendering|SetVisibility _light_l true false)
    (else
      (Rendering|Material|SetScalarParameterValue _lightmat "LightIntensity" 1.0 :!class /Script/Engine.MaterialInstanceDynamic)
      (Rendering|SetVisibility _light_l false false))))

(fn ConstructionScript)

(fn ActivateConstraint
  (params (Constraint :type Physics%20Constraint%20Component%20Object%20Reference) (MainMesh :type Primitive%20Component%20Object%20Reference) (SecondMesh :type Primitive%20Component%20Object%20Reference))
  (Physics|SetSimulatePhysics SecondMesh true)
  (Class|PhysicsConstraintComponent|SetConstrainedComponents Constraint MainMesh "None" SecondMesh "None"))

(fn CloseMesh
  (params (Constraint :type Physics%20Constraint%20Component%20Object%20Reference) (MainMesh :type Primitive%20Component%20Object%20Reference) (SecondMesh :type Primitive%20Component%20Object%20Reference))
  (Physics|SetSimulatePhysics SecondMesh false)
  (Class|PhysicsConstraintComponent|SetConstrainedComponents Constraint 0 "None" 0 "None")
  (Transformation|AttachComponentToComponent SecondMesh MainMesh "None" "KeepWorld" "KeepWorld" "KeepRelative" true)
  (Transformation|SetWorldRotation SecondMesh (Transformation|GetWorldRotation MainMesh) false false))