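; Pickup truck vehicle Blueprint that the third-person character can enter or be killed by.
; A Box overlap kills the character when forward speed is high, otherwise allows entry with the driver seat as attach target until overlap ends.
; While InVehicle is false, overlaps with other wheeled vehicles toggle physics through StartPhysics.
; The U key flags the truck as occupied and starts physics.
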(event OnComponentBeginOverlap(Box)
  (params (OverlappedComponent :type Primitive%20Component%20Object%20Reference) (OtherActor :type Actor%20Object%20Reference) (OtherComp :type Primitive%20Component%20Object%20Reference) (OtherBodyIndex :type Integer) (bFromSweep :type Boolean) (SweepResult :type Hit%20Result%20Structure%20%28by%20ref%29))
  (bind _asthird_person_character (Utilities|Casting|CastToThirdPersonCharacter OtherActor)
    (:then
      (if (> (Math|Float|Absolute(Float) (Class|WheeledVehicleMovementComponent|GetForwardSpeed (Variables|Default|GetVehicleMovement))) 2.5e+02)
        (Default|Death _asthird_person_character _asthird_person_character)
        (else
          (Variables|/Game/ThirdPersonBP/Blueprints/ThirdPersonCharacter.ThirdPersonCharacter_C|SetCanEnterVehicle _asthird_person_character true)
          (Variables|/Game/ThirdPersonBP/Blueprints/ThirdPersonCharacter.ThirdPersonCharacter_C|SetComponentToAttachTo _asthird_person_character (Variables|Default|GetDriverSeat_0))
          (Development|PrintString "Hello"))))
    (:CastFailed
      (if (Utilities|Enum|NotEqual(Enum) (Utilities|GetObjectName OtherActor) (Utilities|GetObjectName self))
        (Utilities|Casting|CastToWheeledVehicle OtherActor)
        (if (not (Variables|Default|GetInVehicle))
          (CallFunction|StartPhysics true))))))

(event OnComponentEndOverlap(Box)
  (params (OverlappedComponent :type Primitive%20Component%20Object%20Reference) (OtherActor :type Actor%20Object%20Reference) (OtherComp :type Primitive%20Component%20Object%20Reference) (OtherBodyIndex :type Integer))
  (bind _asthird_person_character (Utilities|Casting|CastToThirdPersonCharacter OtherActor)
    (:then
      (Variables|/Game/ThirdPersonBP/Blueprints/ThirdPersonCharacter.ThirdPersonCharacter_C|SetCanEnterVehicle _asthird_person_character false))
    (:CastFailed
      (if (Utilities|Enum|NotEqual(Enum) (Utilities|GetObjectName OtherActor) (Utilities|GetObjectName self))
        (Utilities|Casting|CastToWheeledVehicle OtherActor)
        (if (not (Variables|Default|GetInVehicle))
          (CallFunction|StartPhysics false))))))

(event Input|KeyboardEvents|U
  (params (Key :type Key%20Structure))
  (:Pressed
    (Variables|Default|SetInVehicle true)
    (CallFunction|StartPhysics true)))

(fn ConstructionScript)