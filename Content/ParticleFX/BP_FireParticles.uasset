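; Fire particle effect actor that shrinks away while its WaterOn flag is set.
; Tick eases the actor scale toward the default zero target at a constant rate.
; Once X scale drops below 0.1, it deactivates the WaterSystem component a single time, guarded by a Deactivated flag.
; Nothing in this Blueprint sets WaterOn or restores the scale.
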(event EventBeginPlay)

(event EventTick
  (params (DeltaSeconds :type Float%20%28single-precision%29))
  (if (Variables|Default|GetWaterOn)
    (Transformation|SetActorScale3D (Math|Interpolation|VInterptoConstant (Transformation|GetActorScale3D) "0, 0, 0" DeltaSeconds 0.2))
    (if (and (< (.x (Transformation|GetActorScale3D)) 0.1) (not (Variables|Default|GetDeactivated)))
      (Components|Activation|Deactivate (Variables|Default|GetWaterSystem))
      (Variables|Default|SetDeactivated true))))

(fn ConstructionScript)